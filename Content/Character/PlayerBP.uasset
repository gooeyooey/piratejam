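; Player character for a sprite-based pirate game with twin-stick aiming, gun and sword combat, and treasure banking at the player's spawn point.
; Shots spawn bullets and require a manual reload, while timeline-driven sword lunges sphere-trace to kill other players.
; DisableMovement gates movement, aiming and combat until ResetMovement runs.
; Interacting near spawn adds held treasure to the GameMode score, and death teleports the player back after a delay.
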(event Custom|AttackAnim
  ;[1 1 1] attack
  (CallFunction|LungeSprite)
  (bind (_direction _lunge _sword _gun) (Timeline|AttackTL PlayFromStart)
    (:Update
      (Transformation|SetRelativeScale3D (Variables|Default|GetSwordSprite) (Math|Vector|MakeVector (.X (Math|Vector|BreakVector _sword)) (.Y (Math|Vector|BreakVector _sword)) (Utilities|FlipZScale (* (.Z (Math|Vector|BreakVector _sword)) -1.0))))
      (Transformation|SetRelativeScale3D (Variables|Default|GetGunSprite) (Math|Vector|MakeVector (.x (Math|Conversions|ToVector(Float) _gun)) (.y (Math|Conversions|ToVector(Float) _gun)) (Utilities|FlipZScale (.z (Math|Conversions|ToVector(Float) _gun)))))
      (CallFunction|Lunge _lunge))
    (:Finished
      (if (not (Variables|Default|GetDead))
        (CallFunction|ResetMovement)))))

(event Custom|Die
  ;[1 1 1] die
  (if (not (Variables|Default|GetDead))
    (Audio|PlaySoundatLocation "/Game/Sounds/ooh_Cue.ooh_Cue" (Transformation|GetActorLocation) "0, 0, 0" 1.0 1.0 0.0 0 0 0)
    (Variables|Default|SetDead true)
    (Variables|Default|SetDisableMovement true)
    (Sprite|SetFlipbook (Variables|Default|GetCharacterSprite) "/Game/Character/Sprites/Death_Flipbook.Death_Flipbook")
    (Utilities|FlowControl|Delay 1.0)
    (CallFunction|ResetMovement)
    (Transformation|SetActorLocation (Transformation|GetActorLocation (Variables|Default|GetPlayerSpawnPoint)) false false)
    (Variables|Default|SetDead false)))

(event EventBeginPlay
  (bind _asplayer_controller (Utilities|Casting|CastToPlayerController (Pawn|GetController))
    (:then
      (bind _returnvalue (UserInterface|CreateWidget "/Game/UI/player_ui.player_ui_C" _asplayer_controller))
      (UserInterface|Viewport|AddtoPlayerScreen _returnvalue))
    (:CastFailed
      (Development|PrintString "Hello"))))

(event Collision|EventActorBeginOverlap
  (params (OtherActor :type Actor%20Object%20Reference)))

(event EventTick
  (params (DeltaSeconds :type Float%20%28single-precision%29)))

(event EventPossessed
  (params (NewController :type Controller%20Object%20Reference))
  (Utilities|IsValid (Pawn|GetControlledPawn NewController)
    (:Is%20Valid
      (bind _asplayer_controller (Utilities|Casting|CastToPlayerController (Pawn|GetController))
        (:then
          (bind _returnvalue (UserInterface|CreateWidget "/Game/UI/player_ui.player_ui_C" _asplayer_controller))
          (UserInterface|Viewport|AddtoPlayerScreen _returnvalue))
        (:CastFailed
          (Development|PrintString "Hello"))))))

(event Input|ActionEvents|InputActionInteract
  (params (Key :type Key%20Structure))
  ;[1 1 1] Interact
  (:Pressed
    (if (CallFunction|CheckifNearSpawn)
      (CallFunction|DepositTreasure))))

(event Input|ActionEvents|InputActionShoot
  (params (Key :type Key%20Structure))
  (bind _reloadsprite (Variables|Default|GetReloadSprite))
  ;[1 1 1] shoot
  (:Pressed
    (if (not (Variables|Default|GetDisableMovement))
      (if (Variables|Default|GetLoaded)
        (Class|PaperFlipbookComponent|SetPlaybackPositioninFrames (Variables|Default|GetCharacterSprite) 0 false)
        (Components|Timeline|SetPlayRate (Variables|Default|GetCharacterSprite) 0.0)
        (Variables|Default|SetLoaded false)
        (Variables|Default|SetDisableMovement true)
        (Game|SpawnActorfromClass "/Game/Character/Bullet.Bullet_C" (Math|Transform|MakeTransform (Transformation|GetActorLocation) (Math|Conversions|RotationFromXVector (Variables|Default|GetAimDirection)) "1,1,1") "AlwaysSpawn" self 0)
        (Audio|PlaySound2D "/Game/StarterContent/Audio/Explosion01.Explosion01" 1.0 1.0 0.0 0 0)
        (bind _newtrack_0 (Timeline|GunTL PlayFromStart)
          (:Update
            (Transformation|SetRelativeRotation (Variables|Default|GetGunSprite) (Math|Rotator|MakeRotator 8e+01 0.0 (Utilities|FlipZScale _newtrack_0)) false false))
          (:Finished
            (CallFunction|ResetMovement)))
        (else
          (Variables|Default|SetDisableMovement true)
          (Class|PaperFlipbookComponent|SetPlaybackPositioninFrames _reloadsprite 0 false)
          (Development|SetHiddeninGame _reloadsprite false false)
          (Timeline|reloadTL PlayFromStart
            (:Update
              (if (Variables|Default|GetLoaded)
                (Timeline|reloadTL Stop)))
            (:Finished
              (Variables|Default|SetLoaded true)
              (CallFunction|ResetMovement))))))))

(event Input|ActionEvents|InputActionAttack
  (params (Key :type Key%20Structure))
  ;[1 1 1] attack
  (:Pressed
    (CallFunction|Attack)))

(event Input|AxisEvents|InputAxisMoveUp
  (params (AxisValue :type Float%20%28single-precision%29))
  ;[1 1 1] move
  (if (not (Variables|Default|GetDisableMovement))
    (Pawn|Input|AddMovementInput "1.000000,0.000000, 0" AxisValue false)
    (CallFunction|WalkAnim)))

(event Input|AxisEvents|InputAxisMoveRight
  (params (AxisValue :type Float%20%28single-precision%29))
  ;[1 1 1] move
  (if (not (Variables|Default|GetDisableMovement))
    (Pawn|Input|AddMovementInput "0,1.000000, 0" AxisValue false)))

(event Input|AxisEvents|InputAxisAimUp
  (params (AxisValue :type Float%20%28single-precision%29))
  ;[1 1 1] aim
  (CallFunction|SetAimDirection))

(fn ConstructionScript)

(fn SetAimDirection
  (bind _returnvalue (Input|AxisValues|GetAimUp))
  (bind _returnvalue_2 (Input|AxisValues|GetAimRight))
  (bind _returnvalue_3 (* _returnvalue -1.0))
  (bind _returnvalue_4 (Math|Vector|MakeVector _returnvalue_3 _returnvalue_2 0.0))
  (if (and (not (Math|Vector|Equal(Vector) _returnvalue_4 "0, 0, 0" 0.5)) (not (Variables|Default|GetDisableMovement)))
    (bind _output_get (Variables|Default|SetAimDirection (Math|Vector|Normalize _returnvalue_4)))
    (Transformation|SetWorldRotation (Variables|Default|GetArrow1) (Math|Conversions|RotationFromXVector _output_get) false false)
    (Transformation|SetRelativeScale3D (Variables|Default|GetGunSprite) (Math|Vector|MakeVector 0.75 0.75 (Math|Float|SelectFloat -0.75 0.75 (>= (Input|AxisValues|GetAimRight) 0.0))))))

(fn Attack
  (if (not (or (Variables|Default|GetAttacking) (Variables|Default|GetDisableMovement)))
    (Variables|Default|SetAttacking true)
    (Variables|Default|SetDisableMovement true)
    (Development|SetHiddeninGame (Variables|Default|GetSwordSprite) false false)
    (CallFunction|AttackAnim)))

(fn AddtoHeldTreasure
  (params (treasureValue :type Integer))
  (bind _output_get (Variables|Default|SetHeldTreasure (+ (Variables|Default|GetHeldTreasure) treasureValue)))
  (Audio|PlaySoundatLocation "/Game/Sounds/coinGet_Cue.coinGet_Cue" (Transformation|GetActorLocation) "0, 0, 0" 1.0 1.0 0.0 0 0 0))

(fn DepositTreasure
  (bind _playerindex (Variables|Default|GetPlayerIndex))
  (bind _aspirate_game_mode (Utilities|Casting|CastToPirateGameMode (Game|GetGameMode)))
  (Utilities|Array|SetArrayElem (Variables|/Game/PirateGameMode.PirateGameMode_C|GetPlayerScores _aspirate_game_mode) _playerindex (+ (Utilities|Array|Get(acopy) (Variables|/Game/PirateGameMode.PirateGameMode_C|GetPlayerScores _aspirate_game_mode) _playerindex) (Variables|Default|GetHeldTreasure)))
  (Development|PrintString (Utilities|String|ToString(Integer) (Utilities|Array|Get(acopy) (Variables|/Game/PirateGameMode.PirateGameMode_C|GetPlayerScores _aspirate_game_mode) _playerindex)))
  (Variables|Default|SetHeldTreasure 0))

(fn CheckifNearSpawn
  (return (< (Math|Vector|Distance(Vector) (Transformation|GetActorLocation) (Transformation|GetActorLocation (Variables|Default|GetPlayerSpawnPoint))) 2.5e+02)))

(fn WalkAnim
  (bind _returnvalue (Input|AxisValues|GetMoveUp))
  (bind _returnvalue_2 (Input|AxisValues|GetMoveRight))
  (bind _returnvalue_3 (Math|Float|Absolute(Float) _returnvalue))
  (bind _returnvalue_4 (Math|Float|Absolute(Float) _returnvalue_2))
  (bind _returnvalue_5 (+ _returnvalue_3 _returnvalue_4))
  (bind _returnvalue_6 (Math|Float|MapRangeClamped _returnvalue_5 0.0 2.0 0.0 1.0))
  (if (== _returnvalue_6 0.0)
    (Class|PaperFlipbookComponent|SetPlaybackPositioninFrames (Variables|Default|GetCharacterSprite) 0 false)
    (else
      (Components|Timeline|SetPlayRate (Variables|Default|GetCharacterSprite) _returnvalue_6)
      (Transformation|SetRelativeScale3D (Variables|Default|GetCharacterSprite) (Math|Vector|MakeVector (Math|Float|SelectFloat 1.0 -1.0 (> (Input|AxisValues|GetMoveRight) 0.0)) 1.0 1.0)))))

(fn Lunge
  (params (lungeSpeed :type Float%20%28single-precision%29))
  (bind _returnvalue (Transformation|GetActorLocation))
  (Character|LaunchCharacter (* (Variables|Default|GetAimDirection) lungeSpeed) true true)
  (if (> lungeSpeed 2e+02)
    (bind (_outhits _returnvalue_2) (Collision|MultiSphereTraceForObjects _returnvalue (+ _returnvalue (* (Variables|Default|GetAimDirection) (Variables|Default|GetAttackRange))) (Variables|Default|GetAttackRadius) (Utilities|Array|MakeArray "ObjectTypeQuery3") false 0 "None"))
    (if _returnvalue_2
      (bind _array_element (Utilities|Array|ForEachLoopwithBreak _outhits)
        (:LoopBody
          (bind _asplayer_bp (Utilities|Casting|CastToPlayerBP (.HitActor (Collision|BreakHitResult _array_element))))
          (CallFunction|Die _asplayer_bp))))))

(fn LungeSprite
  (Transformation|SetRelativeScale3D (Variables|Default|GetCharacterSprite) (Math|Vector|MakeVector (Math|Float|SelectFloat 1.0 -1.0 (> (Input|AxisValues|GetAimRight) 0.0)) 1.0 1.0))
  (Sprite|SetFlipbook (Variables|Default|GetCharacterSprite) "/Game/Character/Sprites/Lunge_Flipbook.Lunge_Flipbook"))

(fn ResetMovement
  (Variables|Default|SetDisableMovement false)
  (Variables|Default|SetAttacking false)
  (Development|SetHiddeninGame (Variables|Default|GetSwordSprite) true false)
  (Sprite|SetFlipbook (Variables|Default|GetCharacterSprite) "/Game/Character/Sprites/testRun.testRun")
  (Development|SetHiddeninGame (Variables|Default|GetReloadSprite) true false))